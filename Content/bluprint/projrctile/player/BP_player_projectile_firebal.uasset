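; Player fireball projectile Blueprint that gives its flipbook sprite a glowing tint.
; On BeginPlay, after the parent logic, it creates a dynamic instance of the custom unlit sprite material on the PaperFlipbook and stores it as GlowFirebal.
; It then sets that material's flash multiplier and color parameters for a strong red glow.
; The Blueprint adds no movement or hit logic of its own.
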(event EventBeginPlay
  (|CallParentFunction)
  (bind _returnvalue (Rendering|Material|CreateDynamicMaterialInstance (Variables|Default|GetPaperFlipbook) 0 "/Game/materials/M_custom_unlit_sprite.M_custom_unlit_sprite" "None" :!class /Script/Engine.PrimitiveComponent))
  (Variables|Default|Setglow%20firebal _returnvalue)
  (Rendering|Material|SetScalarParameterValue (Variables|Default|Getglow%20firebal) "FLASHmultiplayer" 5e+01 :!class /Script/Engine.MaterialInstanceDynamic)
  (Rendering|Material|SetVectorParameterValue (Variables|Default|Getglow%20firebal) "FLASHCOLOR" "(R=1.000000,G=0.000000,B=0.047890,A=1.000000)" :!class /Script/Engine.MaterialInstanceDynamic))

(event Collision|EventActorBeginOverlap
  (params (OtherActor :type Actor%20Object%20Reference))
  (|CallParentFunction OtherActor) ; This node is disabled and will not be called.\nDrag off pins to build functionality.
)

(event EventTick
  (params (DeltaSeconds :type Float%20%28single-precision%29))
  (|CallParentFunction DeltaSeconds) ; This node is disabled and will not be called.\nDrag off pins to build functionality.
)

(fn ConstructionScript
  (|CallParentFunction))