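; Base action character Blueprint with a sprite that takes damage, flashes when hit and is destroyed on death.
; AnyDamage passes damage to the BPCVitality component, then either destroys the actor if it is dead or triggers a grey flash.
; The flash drives intensity and color parameters on a dynamic sprite material created at BeginPlay, with a rate-adjustable timeline fading the intensity back to zero.
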(event Custom|trigger%20flash
  (params (FLASHmultiplayer :type Float%20%28single-precision%29) (FLASHcolor :type Linear%20Color%20Structure))
  (Rendering|Material|SetScalarParameterValue (Variables|Default|GetDYNAMICspritematerial) "FLASHmultiplayer" FLASHmultiplayer :!class /Script/Engine.MaterialInstanceDynamic)
  (Rendering|Material|SetVectorParameterValue (Variables|Default|GetDYNAMICspritematerial) "FLASHcolor" FLASHcolor :!class /Script/Engine.MaterialInstanceDynamic)
  (Components|Timeline|SetPlayRate (Variables|Default|Getfade%20sprite%20flash) (Variables|Default|Getflash%20Rate))
  (bind _alpa (Timeline|fade%20sprite%20flash PlayFromStart)
    (:Update
      (Rendering|Material|SetScalarParameterValue (Variables|Default|GetDYNAMICspritematerial) "FLASHmultiplayer" (Math|Float|Lerp FLASHmultiplayer 0.0 _alpa) :!class /Script/Engine.MaterialInstanceDynamic))))

(event EventBeginPlay
  (bind _returnvalue (Rendering|Material|CreateDynamicMaterialInstance (Variables|Default|GetSprite) 0 0 "None" :!class /Script/Engine.PrimitiveComponent))
  (Variables|Default|SetDYNAMICspritematerial _returnvalue))

(event Collision|EventActorBeginOverlap
  (params (OtherActor :type Actor%20Object%20Reference)))

(event EventTick
  (params (DeltaSeconds :type Float%20%28single-precision%29)))

(event Game|Damage|EventAnyDamage
  (params (Damage :type Float%20%28single-precision%29) (DamageType :type Damage%20Type%20Object%20Reference) (InstigatedBy :type Controller%20Object%20Reference) (DamageCauser :type Actor%20Object%20Reference))
  (Default|ReceiveDAMGE (Variables|Default|GetBP_C_vitality) Damage)
  (if (Variables|/Game/bluprint/components/BP_C_vitality.BP_C_vitality_C|GetisDEAD (Variables|Default|GetBP_C_vitality))
    (Actor|DestroyActor)
    (else
      (CallFunction|TriggerFlash 3e+01 "(R=0.627083,G=0.627083,B=0.627083,A=1.000000)"))))

(fn ConstructionScript)