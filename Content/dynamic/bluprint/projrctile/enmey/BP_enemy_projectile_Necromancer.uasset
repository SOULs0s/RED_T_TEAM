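; Necromancer enemy projectile Blueprint that adds visual and audio dressing on top of its parent class's behavior.
; BeginPlay gives the flipbook a dynamic unlit sprite material with a red flash tint at full strength.
; Tick watches the current flipbook and uses a resettable DoOnce to play a sigh cue each time the attack effect animation starts.
; Destroyed calls the parent, then a play-sound node with no sound assigned.
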(event EventBeginPlay
  (|CallParentFunction)
  (bind _returnvalue (Rendering|Material|CreateDynamicMaterialInstance (Variables|Default|GetPaperFlipbook) 0 "/Game/static/materials/MI_custom_unlit_sprite.MI_custom_unlit_sprite" "None" :!class /Script/Engine.PrimitiveComponent))
  (Variables|Default|SetNewVar _returnvalue)
  (Rendering|Material|SetScalarParameterValue (Variables|Default|GetNewVar) "FLASHmultiplayer" 1.0 :!class /Script/Engine.MaterialInstanceDynamic)
  (Rendering|Material|SetVectorParameterValue (Variables|Default|GetNewVar) "FLASHcolor" "(R=1.000000,G=0.008761,B=0.000000,A=1.000000)" :!class /Script/Engine.MaterialInstanceDynamic))

(event Collision|EventActorBeginOverlap
  (params (OtherActor :type Actor%20Object%20Reference))
  (|CallParentFunction OtherActor) ; This node is disabled and will not be called.\nDrag off pins to build functionality.
)

(event EventTick
  (params (DeltaSeconds :type Float%20%28single-precision%29))
  (|CallParentFunction DeltaSeconds)
  (if (== (Class|PaperFlipbookComponent|GetFlipbook (Variables|Default|GetPaperFlipbook)) "/Game/static/assets/fx/Necromancer/flipbook/spr_NecromancerAttackEffect_strip48.spr_NecromancerAttackEffect_strip48")
    (Utilities|FlowControl|DoOnce false :!label _label
      (:Completed
        (Audio|PlaySoundatLocation "/Game/dynamic/audio/SFX/enemy_vfx/Fae_Sigh_Cue.Fae_Sigh_Cue" (Transformation|GetActorLocation) "0, 0, 0" 1.0 1.0 0.0 0 0 0 0)))
    (else
      (goto _label Reset))))

(event EventDestroyed
  (|CallParentFunction)
  (Audio|PlaySoundatLocation 0 (Transformation|GetActorLocation) "0, 0, 0" 1.0 1.0 0.0 0 0 0 0))

(fn ConstructionScript
  (|CallParentFunction))