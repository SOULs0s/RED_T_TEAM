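; Base projectile Blueprint that damages action characters of an opposing faction and destroys itself on impact.
; A blocking hit on its Sphere spawns a hit effect actor, plays a plasma blaster sound and destroys the projectile.
; A Sphere overlap with a character of a different Faction applies the projectile's damage before the same impact sequence, while same-faction characters and other overlapping actors are ignored.
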(event OnComponentHit(Sphere)
  (params (HitComponent :type Primitive%20Component%20Object%20Reference) (OtherActor :type Actor%20Object%20Reference) (OtherComp :type Primitive%20Component%20Object%20Reference) (NormalImpulse :type Vector :default "0, 0, 0") (Hit :type Hit%20Result%20Structure%20%28by%20ref%29))
  ;[1 1 1] play hit effect
  (Game|SpawnActorfromClass "/Game/dynamic/bluprint/fx/BP_fx_shoothit.BP_fx_shoothit_C" (Math|Transform|MakeTransform (Transformation|GetActorLocation) (Transformation|GetActorRotation) "1.000000,1.000000,1.000000") "AlwaysSpawn" "MultiplyWithRoot" 0 0)
  (Audio|PlaySoundatLocation "/Game/dynamic/audio/SFX/player_vfx/plasmablaster-37114_Cue.plasmablaster-37114_Cue" (Transformation|GetActorLocation) "0, 0, 0" 1.0 1.0 0.0 0 0 0 0)
  (Actor|DestroyActor))

(event OnComponentBeginOverlap(Sphere)
  (params (OverlappedComponent :type Primitive%20Component%20Object%20Reference) (OtherActor :type Actor%20Object%20Reference) (OtherComp :type Primitive%20Component%20Object%20Reference) (OtherBodyIndex :type Integer) (bFromSweep :type Boolean) (SweepResult :type Hit%20Result%20Structure%20%28by%20ref%29))
  (bind _asbp_action_charactor_base (Utilities|Casting|CastToBP_action_charactor_base OtherActor))
  (if (Utilities|Enum|NotEqual(Enum) (Variables|/Game/dynamic/bluprint/charactor/BP_action_charactor_base.BP_action_charactor_base_C|Getfaction _asbp_action_charactor_base) (Variables|Default|Getfaction))
    (Game|Damage|ApplyDamage _asbp_action_charactor_base (Variables|Default|GetprojrctileDAMGE) 0 self)
    ;[1 1 1] play hit effect
    (Game|SpawnActorfromClass "/Game/dynamic/bluprint/fx/BP_fx_shoothit.BP_fx_shoothit_C" (Math|Transform|MakeTransform (Transformation|GetActorLocation) (Transformation|GetActorRotation) "1.000000,1.000000,1.000000") "AlwaysSpawn" "MultiplyWithRoot" 0 0)
    (Audio|PlaySoundatLocation "/Game/dynamic/audio/SFX/player_vfx/plasmablaster-37114_Cue.plasmablaster-37114_Cue" (Transformation|GetActorLocation) "0, 0, 0" 1.0 1.0 0.0 0 0 0 0)
    (Actor|DestroyActor)))

(event EventBeginPlay)

(event Collision|EventActorBeginOverlap
  (params (OtherActor :type Actor%20Object%20Reference)))

(event EventTick
  (params (DeltaSeconds :type Float%20%28single-precision%29)))

(fn ConstructionScript)