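; Necromancer enemy Blueprint that attacks with a projectile and leaves a death effect.
; Shoot Soul plays the attack animation as an override on the animation component's AnimInstance.
; A separate spawn projectile function fires the Necromancer projectile from the Shootpos transform; neither function is called within this Blueprint.
; On Destroyed, it runs the parent logic and spawns the death FX actor at its own location and rotation.
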(event EventBeginPlay
  (|CallParentFunction) ; This node is disabled and will not be called.\nDrag off pins to build functionality.
)

(event Collision|EventActorBeginOverlap
  (params (OtherActor :type Actor%20Object%20Reference))
  (|CallParentFunction OtherActor) ; This node is disabled and will not be called.\nDrag off pins to build functionality.
)

(event EventTick
  (params (DeltaSeconds :type Float%20%28single-precision%29))
  (|CallParentFunction DeltaSeconds) ; This node is disabled and will not be called.\nDrag off pins to build functionality.
)

(event EventDestroyed
  (|CallParentFunction)
  (Game|SpawnActorfromClass "/Game/dynamic/bluprint/fx/BP_fx_enemy_necro_dead.BP_fx_enemy_necro_dead_C" (Math|Transform|MakeTransform (Transformation|GetActorLocation) (Transformation|GetActorRotation) "1.000000,1.000000,1.000000") "AlwaysSpawn" "MultiplyWithRoot" 0 0))

(fn ConstructionScript
  (|CallParentFunction))

(fn ShootSoul
  (Class|PaperZDAnimInstance|PlayAnimationOverride (Variables|/Script/PaperZD.PaperZDAnimationComponent|GetAnimInstance (Variables|Default|GetAnimationComponent)) "/Game/dynamic/bluprint/charactor/enemy/Necromancer/AnimSequences/Necromancer_attack.Necromancer_attack" "DefaultSlot" 1.0 0.0))

(fn SpawnProjectile
  (bind _shootpos (Variables|Default|Getshootpos))
  (Game|SpawnActorfromClass "/Game/dynamic/bluprint/projrctile/enmey/BP_enemy_projectile_Necromancer.BP_enemy_projectile_Necromancer_C" (Math|Transform|MakeTransform (Transformation|GetWorldLocation _shootpos) (Transformation|GetWorldRotation _shootpos) "1.000000,1.000000,1.000000") "AlwaysSpawn" "MultiplyWithRoot" 0 0))