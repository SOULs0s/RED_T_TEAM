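; Flying demon enemy that hands the player to its AI controller as a target and leaves a death effect.
; The first player overlap with its aggro range passes that player to AIC_fliyingDemon, guarded by a DoOnce.
; A movetowards event applies movement input and snaps the actor to one of two opposite facings based on the direction's X sign.
; On destruction it spawns the death FX actor in its place.
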(event OnComponentBeginOverlap(aggrorange)
  (params (OverlappedComponent :type Primitive%20Component%20Object%20Reference) (OtherActor :type Actor%20Object%20Reference) (OtherComp :type Primitive%20Component%20Object%20Reference) (OtherBodyIndex :type Integer) (bFromSweep :type Boolean) (SweepResult :type Hit%20Result%20Structure%20%28by%20ref%29))
  (bind _asbp_player (Utilities|Casting|CastToBP_player OtherActor))
  (Utilities|FlowControl|DoOnce false
    (:Completed
      (bind _asaic_fliying_demon (Utilities|Casting|CastToAIC_fliyingDemon (AI|GetAIController self)))
      (Default|SetTargetPlayer _asaic_fliying_demon _asbp_player))))

(event Custom|move%20towards
  (params (WorldDirection :type Vector) (ScaleValue :type Float%20%28single-precision%29))
  (Pawn|Input|AddMovementInput WorldDirection ScaleValue false)
  (Transformation|SetActorRotation (select (< (.X (Math|Vector|BreakVector WorldDirection)) 0.0) "0, 0, 0" "0.000000,180.000000,0.000000")))

(event EventBeginPlay
  (|CallParentFunction) ; This node is disabled and will not be called.\nDrag off pins to build functionality.
)

(event Collision|EventActorBeginOverlap
  (params (OtherActor :type Actor%20Object%20Reference))
  (|CallParentFunction OtherActor) ; This node is disabled and will not be called.\nDrag off pins to build functionality.
)

(event EventTick
  (params (DeltaSeconds :type Float%20%28single-precision%29))
  (|CallParentFunction DeltaSeconds) ; This node is disabled and will not be called.\nDrag off pins to build functionality.
)

(event EventDestroyed
  (|CallParentFunction)
  (Game|SpawnActorfromClass "/Game/dynamic/bluprint/fx/BP_fx_enemy_fliying_dead.BP_fx_enemy_fliying_dead_C" (Math|Transform|MakeTransform (Transformation|GetActorLocation) (Transformation|GetActorRotation) "1.000000,1.000000,1.000000") "AlwaysSpawn" "MultiplyWithRoot" 0 0))

(fn ConstructionScript
  (|CallParentFunction))