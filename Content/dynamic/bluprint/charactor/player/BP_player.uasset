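; Player character for a side-scrolling shooter, with Enhanced Input movement, wall slide and jump, and regular and fireball shots.
; A forward trace while falling caps slide speed, enabling wall jumps that briefly drop falling friction.
; Shots spend per-type energy refunded after retriggerable delays, spawning from normal or wall-slide muzzles.
; Damage, including enemy capsule overlaps, triggers knockback, a hurt animation that blocks moving and shooting, and temporary invincibility by ignoring pawn collision.
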(event OnComponentBeginOverlap(CapsuleComponent)
  (params (OverlappedComponent :type Primitive%20Component%20Object%20Reference) (OtherActor :type Actor%20Object%20Reference) (OtherComp :type Primitive%20Component%20Object%20Reference) (OtherBodyIndex :type Integer) (bFromSweep :type Boolean) (SweepResult :type Hit%20Result%20Structure%20%28by%20ref%29))
  (bind _asbp_enemy_base (Utilities|Casting|CastToBP_enemy_base OtherActor))
  (if (== (Variables|/Script/Engine.Character|GetCapsuleComponent _asbp_enemy_base) OtherComp)
    (Game|Damage|ApplyDamage self (Variables|damige|Getoverlap%20Damage) 0 _asbp_enemy_base)))

(event Custom|trigger%20invinc
  (Collision|SetCollisionResponsetoChannel (Variables|Default|GetCapsuleComponent) "ECC_Pawn" "ECR_Ignore")
  (Utilities|FlowControl|RetriggerableDelay (Variables|damige|Getinv%20Duration))
  (Collision|SetCollisionResponsetoChannel (Variables|Default|GetCapsuleComponent) "ECC_Pawn" "ECR_Overlap"))

(event Custom|trigger%20anim
  (Variables|shooting|SetIS_shooting true)
  (Utilities|FlowControl|RetriggerableDelay (Variables|shooting|Getshoot_anim_Duration))
  (Variables|shooting|SetIS_shooting false))

(event Input|EnhancedActionEvents|EnhancedInputActionIA_jump
  (params (ActionValue :type Boolean) (ElapsedSeconds :type Float%20%28double-precision%29) (TriggeredSeconds :type Float%20%28double-precision%29) (InputAction :type Input%20Action%20Object%20Reference :default "/Game/dynamic/input/action/IA_jump.IA_jump"))
  (:Started
    (if (Variables|walljump|Getis%20wall%20sliding)
      (Variables|/Script/Engine.CharacterMovementComponent|SetFallingLateralFriction (Variables|Character|GetCharacterMovement) 0.0)
      (Character|LaunchCharacter (Math|Vector|MakeVector (* (.x (Transformation|GetActorForwardVector)) -1.0 (Variables|walljump|Getwall%20jump%20poewr)) 0.0 (Variables|walljump|Getwall%20jump%20power%20Z)) true true)
      (Utilities|FlowControl|RetriggerableDelay (Variables|walljump|Getwall%20jump%20lock))
      (Variables|/Script/Engine.CharacterMovementComponent|SetFallingLateralFriction (Variables|Character|GetCharacterMovement) (Variables|Default|Getbase%20Falling%20Lateral%20Friction))
      (else
        (Character|Jump))))
  (:Canceled
    (Character|StopJumping :!label _label))
  (:Completed
    (goto _label)))

(event Input|EnhancedActionEvents|EnhancedInputActionIA_move
  (params (ActionValue :type Float%20%28double-precision%29) (ElapsedSeconds :type Float%20%28double-precision%29) (TriggeredSeconds :type Float%20%28double-precision%29) (InputAction :type Input%20Action%20Object%20Reference :default "/Game/dynamic/input/action/IA_move.IA_move"))
  (if (not (Variables|damige|GetIS%20hurt))
    (Pawn|Input|AddMovementInput "1.000000,0.000000,0.000000" ActionValue false)
    (Pawn|SetControlRotation (Pawn|GetController) (select (>= ActionValue 0.0) (Math|Rotator|MakeRotator 0.0 0.0 0.0) (Math|Rotator|MakeRotator 0.0 0.0 1.8e+02)))))

(event Input|EnhancedActionEvents|EnhancedInputActionIA_charge_shoot
  (params (ActionValue :type Boolean) (ElapsedSeconds :type Float%20%28double-precision%29) (TriggeredSeconds :type Float%20%28double-precision%29) (InputAction :type Input%20Action%20Object%20Reference :default "/Game/dynamic/input/action/IA_charge_shoot.IA_charge_shoot"))
  (:Started
    (if (not (Variables|damige|GetIS%20hurt))
      (if (> (Variables|shooting|Getshooting%20energy%20firebal) 0)
        (Math|Integer|DecrementInt (Variables|shooting|Getshooting%20energy%20firebal)
          (:%20%20
            (Utilities|FlowControl|Sequence
              (:then_0
                (goto _label Open))
              (:then_1
                _)
              (:then_2
                (Utilities|FlowControl|RetriggerableDelay (Variables|shooting|Getfier%20rate%20fierbal))
                (shooting|FireRateFirebal))
              (:then_3
                (goto _label Close)))
            (Utilities|FlowControl|Gate true :!label _label
              (:Exit
                (CallFunction|SpawnProjectile "/Game/dynamic/bluprint/projrctile/player/BP_player_projectile_firebal.BP_player_projectile_firebal_C")
                (CallFunction|TriggerFlash 7e+01 "(R=1.000000,G=0.040151,B=0.000000,A=1.000000)")))))))))

(event Input|EnhancedActionEvents|EnhancedInputActionIA_SHOOT
  (params (ActionValue :type Boolean) (ElapsedSeconds :type Float%20%28double-precision%29) (TriggeredSeconds :type Float%20%28double-precision%29) (InputAction :type Input%20Action%20Object%20Reference :default "/Game/dynamic/input/action/IA_SHOOT.IA_SHOOT"))
  (:Started
    (if (not (Variables|damige|GetIS%20hurt))
      (if (> (Variables|shooting|Getshooting%20energy%20regulr) 0)
        (Math|Integer|DecrementInt (Variables|shooting|Getshooting%20energy%20regulr)
          (:%20%20
            (Utilities|FlowControl|Sequence
              (:then_0
                (goto _label Open))
              (:then_1
                _)
              (:then_2
                (Utilities|FlowControl|RetriggerableDelay (Variables|shooting|Getfair%20rate%20regulr))
                (shooting|FireRateRegular))
              (:then_3
                (goto _label Close)))
            (Utilities|FlowControl|Gate true :!label _label
              (:Exit
                (CallFunction|SpawnProjectile "/Game/dynamic/bluprint/projrctile/player/BP_player_projectile_regulr.BP_player_projectile_regulr_C")))))))))

(event EventBeginPlay
  (|CallParentFunction)
  (Utilities|FlowControl|Sequence
    (:then_0
      (bind _asplayer_controller (Utilities|Casting|CastToPlayerController (Pawn|GetController)))
      (Input|AddMappingContext (PlayerController|LocalPlayerSubsystems|GetEnhancedInputLocalPlayerSubsystem _asplayer_controller) "/Game/dynamic/input/IMC_action.IMC_action" 0 "(bIgnoreAllPressedKeysUntilRelease=True,bForceImmediately=False,bNotifyUserSettings=False)"))
    (:then_1
      (Variables|Default|Setbase%20Falling%20Lateral%20Friction (Variables|/Script/Engine.CharacterMovementComponent|GetFallingLateralFriction (Variables|Character|GetCharacterMovement))))))

(event Game|Damage|EventAnyDamage
  (params (Damage :type Float%20%28single-precision%29) (DamageType :type Damage%20Type%20Object%20Reference) (InstigatedBy :type Controller%20Object%20Reference) (DamageCauser :type Actor%20Object%20Reference))
  (|CallParentFunction Damage DamageType InstigatedBy DamageCauser)
  (CallFunction|TriggerInvinc)
  (Variables|/Script/Engine.CharacterMovementComponent|SetFallingLateralFriction (Variables|Character|GetCharacterMovement) 0.0)
  (Character|LaunchCharacter (Math|Vector|MakeVector (* (Math|Float|SelectFloat -1.0 1.0 (>= (.x (Math|Vector|GetForwardVector (Math|Rotator|FindLookatRotation (Transformation|GetActorLocation) (Transformation|GetActorLocation DamageCauser)))) 0.0)) (Variables|knockback|Getknockback%20power_X)) 0.0 (Variables|knockback|Getknockback%20power_Z)) true true)
  (Class|PaperZDAnimInstance|JumptoNode (Variables|/Script/PaperZD.PaperZDAnimationComponent|GetAnimInstance (Variables|Default|GetAnimationComponent)) "jump hurt" "None")
  (Variables|damige|SetIS%20hurt true)
  (Utilities|FlowControl|Sequence
    (:then_0
      (Utilities|FlowControl|RetriggerableDelay (Variables|damige|Getinv%20Duration))
      (Variables|/Script/Engine.CharacterMovementComponent|SetFallingLateralFriction (Variables|Character|GetCharacterMovement) (Variables|Default|Getbase%20Falling%20Lateral%20Friction)))
    (:then_1
      (Utilities|FlowControl|RetriggerableDelay (Variables|damige|Gethurt%20Duration))
      (Variables|damige|SetIS%20hurt false))))

(event EventTick
  (params (DeltaSeconds :type Float%20%28single-precision%29))
  (bind _returnvalue (Transformation|GetActorLocation))
  (|CallParentFunction 0.0)
  (if (and (<= (.z (Variables|/Script/Engine.MovementComponent|GetVelocity (Variables|Character|GetCharacterMovement))) -5e+01) (> (* (.x (Transformation|GetActorForwardVector)) (Input|EnhancedActionValues|GetIA_move)) 0.0))
    (bind _returnvalue_2 (Collision|LineTraceForObjects _returnvalue (+ _returnvalue (* (Transformation|GetActorForwardVector) (Variables|walljump|Getwall%20tace%20length))) (Utilities|Array|MakeArray "ObjectTypeQuery1") false 0 "None"))
    (if _returnvalue_2
      (Variables|walljump|Setis%20wall%20sliding true)
      (Variables|/Script/Engine.MovementComponent|SetVelocity (Variables|Character|GetCharacterMovement) (Math|Vector|MakeVector (.x (Variables|/Script/Engine.MovementComponent|GetVelocity (Variables|Character|GetCharacterMovement))) (.y (Variables|/Script/Engine.MovementComponent|GetVelocity (Variables|Character|GetCharacterMovement))) (Math|Float|Max(Float) (.z (Variables|/Script/Engine.MovementComponent|GetVelocity (Variables|Character|GetCharacterMovement))) (Variables|walljump|Getwall%20slide%20speed))))
      (else
        (Variables|walljump|Setis%20wall%20sliding false)))
    (else
      (Variables|walljump|Setis%20wall%20sliding false))))

(fn ConstructionScript
  (|CallParentFunction))

(fn FireRateRegular
  (Math|Integer|IncrementInt (Variables|shooting|Getshooting%20energy%20regulr)))

(fn SpawnProjectile
  (params (projectile%20Class :type BP%20Plaayer%20Projectile%20Base%20Class%20Reference))
  (bind _self self)
  (bind _shootpos (Variables|Default|Getshootpos))
  (bind _is_wall_sliding (Variables|walljump|Getis%20wall%20sliding))
  (bind _wall_climb_shoot (Variables|Default|Getwall%20climb%20shoot))
  (bind _returnvalue (select _is_wall_sliding _wall_climb_shoot _shootpos))
  (bind _returnvalue_2 (Transformation|GetWorldTransform _returnvalue))
  (Game|SpawnActorfromClass projectile%20Class (Math|Transform|MakeTransform (.location _returnvalue_2) (.rotation _returnvalue_2) "1.000000,1.000000,1.000000") "AlwaysSpawn" "MultiplyWithRoot" _self _self)
  (CallFunction|TriggerAnim))

(fn FireRateFirebal
  (Math|Integer|IncrementInt (Variables|shooting|Getshooting%20energy%20firebal)))

(fn HandelChargeFlash
  (params (elapsed :type Float%20%28double-precision%29)))