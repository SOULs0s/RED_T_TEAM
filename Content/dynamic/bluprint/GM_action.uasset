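; Game mode that sets up the player HUD and provides player respawning.
; On BeginPlay it caches a PlayerStart actor and adds a WBP_HUD widget to the viewport for the first player controller.
; ReaspawnPlayer spawns the default pawn class at the cached start's location and rotation, ignoring collisions, then has that controller possess it.
; The function does not destroy the previous pawn, and nothing in this file calls it.
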(event EventBeginPlay
  (bind _returnvalue (Actor|GetActorOfClass "/Script/Engine.PlayerStart"))
  (Variables|Default|Setplayer%20start _returnvalue)
  (bind _returnvalue_2 (UserInterface|CreateWidget "/Game/dynamic/widgets/WBP_HUD.WBP_HUD_C" (Game|GetPlayerController 0)))
  (bind _output_get (Variables|Default|SetHUD%20widget _returnvalue_2))
  (UserInterface|Viewport|AddtoViewport _output_get 0))

(event EventTick
  (params (DeltaSeconds :type Float%20%28single-precision%29)))

(fn ConstructionScript)

(fn ReaspawnPlayer
  (bind _player_start (Variables|Default|Getplayer%20start))
  (bind _returnvalue (Transformation|GetActorTransform _player_start))
  (bind _returnvalue_2 (Game|SpawnActorfromClass (Variables|Default|GetDefaultPawnClass) (Math|Transform|MakeTransform (.location _returnvalue) (.rotation _returnvalue) "1.000000,1.000000,1.000000") "AlwaysSpawn" "MultiplyWithRoot" 0 0))
  (Pawn|Possess (Game|GetPlayerController 0) _returnvalue_2))