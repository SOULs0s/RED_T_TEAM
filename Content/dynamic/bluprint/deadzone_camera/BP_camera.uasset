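; BP_camera is a room camera that becomes the player's CurrentCam and view target when the player overlaps its trigger box, or starts inside it.
; The construction script sizes the trigger from exposed transform and extent, and a confines box from room width and height.
; Tick runs X and Z follow macros to move the root, but both currently output zero, leaving their FInterpTo smoothing unconnected.
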(event OnComponentBeginOverlap(playertriggerbox)
  (params (OverlappedComponent :type Primitive%20Component%20Object%20Reference) (OtherActor :type Actor%20Object%20Reference) (OtherComp :type Primitive%20Component%20Object%20Reference) (OtherBodyIndex :type Integer) (bFromSweep :type Boolean) (SweepResult :type Hit%20Result%20Structure%20%28by%20ref%29))
  (bind _asbp_player (Utilities|Casting|CastToBP_player OtherActor))
  (Variables|/Game/dynamic/bluprint/charactor/player/BP_player.BP_player_C|Setcurrent%20cam _asbp_player self)
  (Game|Player|SetViewTargetwithBlend (Game|GetPlayerController 0) self 0.0 "VTBlend_Linear" 0.0 false))

(event EventBeginPlay
  (Utilities|FlowControl|Delay 0.2)
  (bind _asbp_player (Utilities|Casting|CastToBP_player (Game|Player|GetPlayerPawn 0)))
  (for _array_element (Class|Actor|GetOverlappingComponents _asbp_player)
    (if (== _array_element (Variables|Default|Getplayer%20trigger%20box))
      (Variables|/Game/dynamic/bluprint/charactor/player/BP_player.BP_player_C|Setcurrent%20cam _asbp_player self)
      (Game|Player|SetViewTargetwithBlend (Game|GetPlayerController 0) self 0.0 "VTBlend_Linear" 0.0 false))))

(event EventTick
  (params (DeltaSeconds :type Float%20%28single-precision%29))
  (Variables|Default|Setdelta%20time DeltaSeconds)
  (Utilities|CamFollowPlayerX
    (:OUT
      (Utilities|CamFollowPlayerZ
        (:out
          (Transformation|SetWorldLocation (Variables|Default|Getroot) (Math|Vector|MakeVector (Variables|Default|Getcurrent%20cam%20lerping%20pos%20X) (.y (Transformation|GetWorldLocation (Variables|Default|Getroot))) (Variables|Default|Getcurrent%20cam%20lerping%20pos%20Z)) false false))))))

(fn ConstructionScript
  (Transformation|SetRelativeTransform (Variables|Default|Getplayer%20trigger%20box) (Variables|Default|Getplayer%20trigger%20transform) false false)
  (Components|Box|SetBoxExtent (Variables|Default|Getplayer%20trigger%20box) (Variables|Default|Getplayer%20trigger%20extent) true)
  (Components|Box|SetBoxExtent (Variables|Default|Getcamera%20confines%20box) (Math|Vector|MakeVector (Math|Conversions|ToFloat(Integer) (* (* (Variables|Default|Getroom%20width) 8) 119)) 1e+01 (Math|Conversions|ToFloat(Integer) (* (* (Variables|Default|Getroom%20height) 8) 69))) true))