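; BP_C_vitality is a vitality component that tracks health and death state.
; On BeginPlay it sets current health to the maximum.
; ReceiveDAMGE subtracts incoming damage, clamps the result between zero and maximum health, and sets the IsDEAD flag when health reaches zero.
; It only updates its own variables, with no event dispatch or death handling, and Tick is unused.
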(event EventBeginPlay
  (Variables|Default|SetcurrentHEALT (Variables|Default|GetmaxHEALTH)))

(event EventTick
  (params (DeltaSeconds :type Float%20%28single-precision%29)))

(fn ReceiveDAMGE
  (params (damage :type Float%20%28double-precision%29))
  (Variables|Default|SetcurrentHEALT (Math|Float|Clamp(Float) (- (Variables|Default|GetcurrentHEALT) damage) 0.0 (Variables|Default|GetmaxHEALTH)))
  (if (<= (Variables|Default|GetcurrentHEALT) 0.0)
    (Variables|Default|SetisDEAD true)))